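; BP_TestSpawner is an actor that spawns a number of team-assigned template characters when play begins.
; It runs the EQS_TestPoint environment query with itself as querier to gather the spawn points.
; It then loops over the requested count, spawning the character type from its row handle at each point, using the spawner's rotation and team.
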(event `self.ReceiveBeginPlay`
  (bind _returnvalue (`PointsLibrary.GetPoints` "/Game/AI/EQS_TestPoint.EQS_TestPoint" self (`self.Num`)))
  (set `self.Arr` _returnvalue)
  (for _index (range 1 (+ (`self.Num`) 1))
    (`BFL.SpawnTemplateCharacter_WorldContext` (`self.TypeSpawnActor`) (`|GetArrayItem` (`self.Arr`) (- _index 1)) (`self.K2_GetActorRotation`) (`self.Team`))))

(event `self.ReceiveActorBeginOverlap`
  (params (OtherActor :type "Actor Object Reference")))

(event `self.ReceiveTick`
  (params (DeltaSeconds :type "Float (single-precision)")))

(fn `UserConstructionScript`)